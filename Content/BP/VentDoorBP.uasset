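; Keypad-locked vent door actor that swings open once when the correct code is entered.
; On BeginPlay it binds to the Keypad_UI widget's code-entered event, and CheckCode compares entries to CorrectCode, clearing the keypad either way.
; OpenVent runs once, blending the view to the camera's owner while a timeline rotates the Pivot, then returning the view to the player.
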(event Custom|Open%20Vent
  (params (Player :type Character%20Object%20Reference))
  (Utilities|FlowControl|DoOnce false
    (:Completed
      (Utilities|FlowControl|Delay 1.0)
      (Game|Player|SetViewTargetwithBlend (Game|GetPlayerController 0) (Components|GetOwner (Variables|Default|GetCamera)) 1.0 "VTBlend_Linear" 0.0 false)
      (Utilities|FlowControl|Delay 1.0)
      (bind _rotate (Timeline|Timeline_0 Play)
        (:Update
          (Transformation|SetRelativeRotation (Variables|Default|Getpivot) (Math|Rotator|Lerp(Rotator) (Variables|Default|GetNewPos) (Variables|Default|GetCurrentPos) _rotate) false false))
        (:Finished
          (Utilities|FlowControl|Delay 1.0)
          (Game|Player|SetViewTargetwithBlend (Game|GetPlayerController 0) Player 0.0 "VTBlend_Linear" 0.0 false))))))

(event EventBeginPlay
  (bind _askeypad_ui (Utilities|Casting|CastToKeypad_UI (UserInterface|GetUserWidgetObject (Variables|Default|GetWidget))))
  (bind _output_get (Variables|Default|SetKeyPadUI _askeypad_ui))
  (EventDispatchers|BindEventtoCodeEntered _output_get (EventDispatchers|CreateEvent :!event CheckCode)))

(fn ConstructionScript)

(fn CheckCode
  (params (Code%20Entered :type String) (Keypad :type Keypad%20UI%20Object%20Reference))
  (if (Utilities|Enum|Equal(Enum) Code%20Entered (Variables|Default|GetCorrectCode))
    (CallFunction|OpenVent (Game|GetPlayerCharacter 0))
    (Variables|/Game/UI/Keypad_UI.Keypad_UI_C|Setcurrentcode (Variables|Default|GetKeyPadUI) "")
    (else
      (Variables|/Game/UI/Keypad_UI.Keypad_UI_C|Setcurrentcode (Variables|Default|GetKeyPadUI) ""))))