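; Interactable button actor that damages a Destructible_Glass actor set as its owner when the player presses Interact nearby.
; It enables player input on BeginPlay, and a box overlap with BP_PlayerCharacter opens and closes a gate on that input.
; A successful press applies damage to the glass, prints a debug string and holds the Buttonpressed flag true briefly before resetting it.
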(event OnComponentBeginOverlap(Box)
  (params (OverlappedComponent :type Primitive%20Component%20Object%20Reference) (OtherActor :type Actor%20Object%20Reference) (OtherComp :type Primitive%20Component%20Object%20Reference) (OtherBodyIndex :type Integer) (bFromSweep :type Boolean) (SweepResult :type Hit%20Result%20Structure%20%28by%20ref%29))
  (Utilities|Casting|CastToBP_PlayerCharacter OtherActor)
  (Utilities|FlowControl|Gate true) ; enters at Open
)

(event OnComponentEndOverlap(Box)
  (params (OverlappedComponent :type Primitive%20Component%20Object%20Reference) (OtherActor :type Actor%20Object%20Reference) (OtherComp :type Primitive%20Component%20Object%20Reference) (OtherBodyIndex :type Integer))
  (Utilities|Casting|CastToBP_PlayerCharacter OtherActor)
  (Utilities|FlowControl|Gate true) ; enters at Close
)

(event EventBeginPlay
  (Input|EnableInput (Game|GetPlayerController 0)))

(event Input|ActionEvents|InputActionInteract
  (params (Key :type Key%20Structure))
  (:Pressed
    (Utilities|FlowControl|Gate true
      (:Exit
        (bind _asdestructible_glass (Utilities|Casting|CastToDestructible_Glass (Components|GetOwner)))
        (Game|Damage|ApplyDamage _asdestructible_glass 1.0 0 (Game|Player|GetPlayerPawn 0) "/Script/Engine.DamageType")
        (Development|PrintString "Hello")
        (Variables|Default|Setbuttonpressed true)
        (Utilities|FlowControl|Delay 1.0)
        (Variables|Default|Setbuttonpressed false)))))

(fn ConstructionScript)