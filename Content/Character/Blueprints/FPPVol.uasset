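; FPPVol is a trigger volume that switches the player character from third-person to first-person view.
; When a component tagged Player begins overlapping its Box, it casts the owning actor to BP_PlayerCharacter and copies that character's FPP flag.
; If the flag is off, it activates FirstPersonCamera, deactivates ThirdPersonCamera and sets the character's flag.
; The switch is one-way, with no end-overlap handling to restore third person.
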(event OnComponentBeginOverlap(Box)
  (params (OverlappedComponent :type Primitive%20Component%20Object%20Reference) (OtherActor :type Actor%20Object%20Reference) (OtherComp :type Primitive%20Component%20Object%20Reference) (OtherBodyIndex :type Integer) (bFromSweep :type Boolean) (SweepResult :type Hit%20Result%20Structure%20%28by%20ref%29))
  (if (Components|ComponentHasTag OtherComp "Player")
    (bind _asbp_player_character (Utilities|Casting|CastToBP_PlayerCharacter OtherActor))
    (if (Variables|/Game/Character/Blueprints/BP_PlayerCharacter.BP_PlayerCharacter_C|GetFPP _asbp_player_character)
      (Variables|Default|SetFPP true)
      (else
        (Variables|Default|SetFPP false)))
    (if (not (Variables|Default|GetFPP))
      (Components|Activation|SetActive (Variables|/Game/Character/Blueprints/BP_PlayerCharacter.BP_PlayerCharacter_C|GetFirst%20Person%20Camera _asbp_player_character) true false)
      (Components|Activation|SetActive (Variables|/Game/Character/Blueprints/BP_PlayerCharacter.BP_PlayerCharacter_C|GetThird%20Person%20Camera _asbp_player_character) false false)
      (Variables|/Game/Character/Blueprints/BP_PlayerCharacter.BP_PlayerCharacter_C|SetFPP _asbp_player_character true))))

(fn ConstructionScript)